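; Pathfinding grid actor that lets the player pick a start and a goal node by looking and clicking.
; Each tick a visibility trace from the camera converts the impact point to a node index and updates the current node.
; Left clicks alternate between storing that node's position as the start and setting the goal, which triggers CalculatePath.
; A SwitchBlocked call for toggling nodes is present but unconnected.
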(event EventBeginPlay
  (Input|EnableInput (Game|GetPlayerController 0)))

(event EventTick
  (params (DeltaSeconds :type Float%20%28single-precision%29))
  (bind _returnvalue (Game|GetPlayerCameraManager 0))
  (bind _returnvalue_2 (Camera|GetCameraLocation _returnvalue))
  (bind _outhit (Collision|LineTraceByChannel _returnvalue_2 (+ _returnvalue_2 (* (Math|Vector|GetForwardVector (Variables|/Script/Engine.PlayerCameraManager|GetTransformComponent _returnvalue)) 1e+04)) "TraceTypeQuery1" false 0 "None"))
  (bind _returnvalue_3 (Class|PathGrid|ConvertPositiontoNodeIndex (.ImpactPoint (Collision|BreakHitResult _outhit))))
  (bind _output_get (Variables|Default|SetNodeIndex _returnvalue_3))
  (Class|PathGrid|UpdateCurrentNode _output_get))

(event Input|MouseEvents|LeftMouseButton
  (params (Key :type Key%20Structure :default "None"))
  (:Pressed
    (bind _returnvalue (Class|PathGrid|ConvertNodeIndextoPosition (Variables|Default|GetNodeIndex)))
    (if (Variables|Default|GetStartSet)
      (Variables|Default|SetGoal _returnvalue)
      (Variables|Default|SetStartSet false)
      (Class|PathGrid|CalculatePath (Variables|Default|GetStartNode) (Variables|Default|GetGoal))
      (else
        (Variables|Default|SetStartNode _returnvalue)
        (Variables|Default|SetStartSet true)))))

(fn ConstructionScript)